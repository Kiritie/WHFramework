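; BPC_WorldTimer is a component that updates scene lighting for a given sun angle, as used for time of day.
; Its UpdateLight event sets the SunLight's pitch and, when a SkySphere is valid, refreshes that sky's sun direction.
; It then blends the SkyLight cubemap from dusk toward night or noon, using the sign of the angle's sine to pick the target and its magnitude as the blend fraction.
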(event EventUpdateLight
  (params (InLightDirection :type Float%20%28single-precision%29))
  (bind _returnvalue (Math|Trig|Sin(Degrees) InLightDirection))
  (bind _dusktex (Variables|Default|GetDuskTex))
  (bind _sunlight (Variables|Default|GetSunLight))
  (bind _skysphere (Variables|Default|GetSkySphere))
  (bind _skylight (Variables|Default|GetSkyLight))
  (bind _returnvalue_2 (Math|Float|Absolute(Float) _returnvalue))
  (bind _lightcomponent (Variables|/Script/Engine.SkyLight|GetLightComponent _skylight))
  (Utilities|IsValid _sunlight
    (:Is%20Valid
      (Transformation|SetActorRelativeRotation _sunlight (Math|Rotator|MakeRotator 0.0 InLightDirection 0.0))
      (Utilities|IsValid _skysphere
        (:Is%20Valid
          (Default|UpdateSunDirection _skysphere)
          (if (> _returnvalue 0.0)
            (Class|SkyLightComponent|SetCubemapBlend _lightcomponent _dusktex (Variables|Default|GetNightTex) _returnvalue_2)
            (else
              (Class|SkyLightComponent|SetCubemapBlend _lightcomponent _dusktex (Variables|Default|GetNoonTex) _returnvalue_2))))))))